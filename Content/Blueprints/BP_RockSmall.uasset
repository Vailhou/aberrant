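; Small rock actor that plays an impact sound when its mesh is hit hard enough.
; The hit event sums the absolute axes of the normal impulse, then maps that value between a threshold and a maximum to scale volume and pitch.
; A DoOnce reset after a short delay throttles repeated sounds.
; GetPrimitiveComponent exposes a primitive component to callers.
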(event OnComponentHit(Mesh)
  (params (HitComponent :type Primitive%20Component%20Object%20Reference) (OtherActor :type Actor%20Object%20Reference) (OtherComp :type Primitive%20Component%20Object%20Reference) (NormalImpulse :type Vector :default "0, 0, 0") (Hit :type Hit%20Result%20Structure%20%28by%20ref%29))
  (bind (_x _y _z) (Math|Vector|BreakVector NormalImpulse))
  (bind _hitsoundthreshold (Variables|Default|GetHitSoundThreshold))
  (bind _hitsoundmaximpulse (Variables|Default|GetHitSoundMaxImpulse))
  (bind _hitsoundthreshold_2 (Variables|Default|GetHitSoundThreshold))
  (bind _hitsoundmaximpulse_2 (Variables|Default|GetHitSoundMaxImpulse))
  (bind _hitsoundthreshold_3 (Variables|Default|GetHitSoundThreshold))
  (bind _returnvalue (Math|Float|Absolute(Float) _x))
  (bind _returnvalue_2 (Math|Float|Absolute(Float) _y))
  (bind _returnvalue_3 (Math|Float|Absolute(Float) _z))
  (bind _returnvalue_4 (- _hitsoundmaximpulse_2 _hitsoundthreshold_3))
  (bind _returnvalue_5 (+ _returnvalue _returnvalue_2 _returnvalue_3))
  (bind _returnvalue_6 (Math|Float|Clamp(Float) _returnvalue_5 _hitsoundthreshold _hitsoundmaximpulse))
  (bind _returnvalue_7 (- _returnvalue_6 _hitsoundthreshold_2))
  (bind _returnvalue_8 (/ _returnvalue_7 _returnvalue_4))
  (if (> _returnvalue_5 (Variables|Default|GetHitSoundThreshold))
    (Utilities|FlowControl|DoOnce false :!label _label
      (:Completed
        (Audio|PlaySoundatLocation "/Game/Audio/SFX/RockHit/MSS_RockHit.MSS_RockHit" (Transformation|GetWorldLocation (Variables|Default|GetMesh)) "0, 0, 0" (Math|Float|Lerp 0.0 2.0 _returnvalue_8) (Math|Float|Lerp 0.0 0.5 _returnvalue_8) 0.0 "/Game/Audio/SFX/ATT_PhysicsActor.ATT_PhysicsActor" 0 0 0)
        (Utilities|FlowControl|Delay 0.2)
        (goto _label Reset)))))

(fn ConstructionScript)

(fn GetPrimitiveComponent
  (return (Variables|Default|GetPrimitiveComponent)))