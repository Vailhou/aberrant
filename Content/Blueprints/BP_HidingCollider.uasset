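; BP_HidingCollider is a trigger volume that detects when the player enters or leaves a hiding spot.
; Overlap begin and end events on its Collider component react only to actors whose class is exactly BP_FirstPersonCharacter.
; They fire the OnPlayerHide and OnPlayerStopHide event dispatchers respectively, each followed by a debug print, leaving the hiding response to whatever binds to them.
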(event OnComponentBeginOverlap(Collider)
  (params (OverlappedComponent :type Primitive%20Component%20Object%20Reference) (OtherActor :type Actor%20Object%20Reference) (OtherComp :type Primitive%20Component%20Object%20Reference) (OtherBodyIndex :type Integer) (bFromSweep :type Boolean) (SweepResult :type Hit%20Result%20Structure%20%28by%20ref%29))
  (if (== (Utilities|GetClass OtherActor) "/Game/Blueprints/BP_FirstPersonCharacter.BP_FirstPersonCharacter_C")
    (Default|CallOnPlayerHide)
    (Development|PrintString "Player hidden" true true "(R=0.076063,G=1.000000,B=0.000000,A=1.000000)")))

(event OnComponentEndOverlap(Collider)
  (params (OverlappedComponent :type Primitive%20Component%20Object%20Reference) (OtherActor :type Actor%20Object%20Reference) (OtherComp :type Primitive%20Component%20Object%20Reference) (OtherBodyIndex :type Integer))
  (if (== (Utilities|GetClass OtherActor) "/Game/Blueprints/BP_FirstPersonCharacter.BP_FirstPersonCharacter_C")
    (Default|CallOnPlayerStopHide)
    (Development|PrintString "Player stopped hiding" true true "(R=1.000000,G=0.000000,B=0.010379,A=1.000000)")))

(event EventBeginPlay)

(event Collision|EventActorBeginOverlap
  (params (OtherActor :type Actor%20Object%20Reference)))

(event EventTick
  (params (DeltaSeconds :type Float%20%28single-precision%29)))

(fn ConstructionScript)