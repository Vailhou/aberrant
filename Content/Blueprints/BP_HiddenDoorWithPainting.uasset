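; Hidden door Blueprint that slides a dungeon wall open when activated and shut when deactivated.
; A DoorOpen timeline, rate-scaled by PlayTime, offsets the wall along the OpenDirection component's forward vector by up to DistanceAmount.
; Both events start two audio components, which fade out when the timeline finishes.
; A required active/inactive check is defined but returns false on every path and is not called in these graphs.
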(event EventDeactivate
  (bind _audio (Variables|Default|GetAudio))
  (Utilities|FlowControl|Sequence
    (:then_0
      (Audio|Components|Audio|Play _audio 0.0))
    (:then_1
      (bind _amount (Timeline|DoorOpen Reverse)
        (:Update
          (Transformation|SetRelativeLocation (Variables|Default|GetSM_Dungeon_Wall) (* (Math|Float|Lerp 0.0 (Variables|Default|GetDistanceAmount) _amount) (Math|Vector|GetForwardVector (Variables|/Script/Engine.SceneComponent|GetRelativeRotation (Variables|Default|GetOpenDirection)))) false false))
        (:Finished
          (Audio|Components|Audio|FadeOut _audio 0.1 0.0 "Linear" :!class /Script/Engine.AudioComponent))))))

(event EventActivate
  (bind _audio (Variables|Default|GetAudio))
  (Utilities|FlowControl|Sequence
    (:then_0
      (Audio|Components|Audio|Play _audio 0.0))
    (:then_1
      (bind _amount (Timeline|DoorOpen Play)
        (:Update
          (Transformation|SetRelativeLocation (Variables|Default|GetSM_Dungeon_Wall) (* (Math|Float|Lerp 0.0 (Variables|Default|GetDistanceAmount) _amount) (Math|Vector|GetForwardVector (Variables|/Script/Engine.SceneComponent|GetRelativeRotation (Variables|Default|GetOpenDirection)))) false false))
        (:Finished
          (Audio|Components|Audio|FadeOut _audio 0.1 0.0 "Linear" :!class /Script/Engine.AudioComponent))))))

(event EventBeginPlay
  (Components|Timeline|SetPlayRate (Variables|Default|GetDoorOpen) (/ 1.0 (Variables|Default|GetPlayTime))))

(fn ConstructionScript)

(fn CheckIsRequiredActiveandInactive?
  (bind _array_element (Utilities|Array|ForEachLoopwithBreak (Variables|Default|GetRequiredToBeActive))
    (:LoopBody
      (if (not (Utilities|Array|ContainsItem (Variables|Default|GetActivated) _array_element))
        (return false)))
    (:Completed
      (bind _array_element_2 (Utilities|Array|ForEachLoopwithBreak (Variables|Default|GetRequiredToBeInactive))
        (:LoopBody
          (if (Utilities|Array|ContainsItem (Variables|Default|GetActivated) _array_element_2)
            (return false)))
        (:Completed
          (return false))))))