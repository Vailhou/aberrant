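; BP_Door is a sliding door Blueprint that opens on Activate and closes on Deactivate.
; A DoorOpen timeline plays forward or in reverse, with its play rate set at BeginPlay to the inverse of PlayTime.
; Each update moves the Cube in relative space along the OpenDirection component's forward vector, interpolating from zero to DistanceAmount without sweeping.
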(event EventDeactivate
  (bind _amount (Timeline|DoorOpen Reverse)
    (:Update
      (Transformation|SetRelativeLocation (Variables|Default|GetCube) (* (Math|Float|Lerp 0.0 (Variables|Default|GetDistanceAmount) _amount) (Math|Vector|GetForwardVector (Variables|/Script/Engine.SceneComponent|GetRelativeRotation (Variables|Default|GetOpenDirection)))) false false))))

(event EventActivate
  (bind _amount (Timeline|DoorOpen Play)
    (:Update
      (Transformation|SetRelativeLocation (Variables|Default|GetCube) (* (Math|Float|Lerp 0.0 (Variables|Default|GetDistanceAmount) _amount) (Math|Vector|GetForwardVector (Variables|/Script/Engine.SceneComponent|GetRelativeRotation (Variables|Default|GetOpenDirection)))) false false))))

(event EventBeginPlay
  (Components|Timeline|SetPlayRate (Variables|Default|GetDoorOpen) (/ 1.0 (Variables|Default|GetPlayTime))))

(fn ConstructionScript)