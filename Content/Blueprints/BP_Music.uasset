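; Music manager Blueprint that switches between ambient and chase music in response to enemy chases and player death.
; On BeginPlay it loops over every BP_Enemy, binding chase and player distance/death events and spawning the ambient sound.
; Chase handlers crossfade the two audio components, while death fades out chase music using the player's death delay.
; Clamped enemy distance drives the chase music's EffectAmount parameter, increasing it as the enemy gets closer.
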(event EventBeginPlay
  (bind _outactors (Actor|GetAllActorsOfClass "/Game/Blueprints/BP_Enemy.BP_Enemy_C"))
  (bind _output_get (Variables|Default|SetEnemies _outactors))
  (for _array_element _output_get
    (EventDispatchers|BindEventtoOnChaseStarted _array_element (EventDispatchers|CreateEvent :!event StartChase))
    (EventDispatchers|BindEventtoOnChaseEnded _array_element (EventDispatchers|CreateEvent :!event EndChase))
    (bind _returnvalue (Actor|GetActorOfClass "/Game/Blueprints/BP_FirstPersonCharacter.BP_FirstPersonCharacter_C"))
    (EventDispatchers|BindEventtoOnEnemyDistance _returnvalue (EventDispatchers|CreateEvent :!event SetChaseEffectAmount))
    (EventDispatchers|BindEventtoOnDeath _returnvalue (EventDispatchers|CreateEvent :!event Death))
    (Variables|Default|SetDeathFadeOutDuration (Variables|/Game/Blueprints/BP_FirstPersonCharacter.BP_FirstPersonCharacter_C|GetDeathDelay _returnvalue))
    (Audio|SpawnSound2D "/Game/Audio/SFX/Ambient/MSS_Ambient.MSS_Ambient" 1.0 1.0 0.0 0)))

(fn ConstructionScript)

(fn EndChase
  (bind _fadeoutdurationchase (Variables|Default|GetFadeOutDurationChase))
  (Audio|Components|Audio|FadeOut (Variables|Default|GetChaseMusicAudio) _fadeoutdurationchase 0.0 "Linear" :!class /Script/Engine.AudioComponent)
  (Audio|Components|Audio|FadeIn (Variables|Default|GetAmbientMusicAudio) _fadeoutdurationchase 1.0 0.0 "Linear" :!class /Script/Engine.AudioComponent))

(fn StartChase
  (bind _fadeindurationchase (Variables|Default|GetFadeInDurationChase))
  (Audio|Components|Audio|FadeOut (Variables|Default|GetAmbientMusicAudio) _fadeindurationchase 0.0 "Linear" :!class /Script/Engine.AudioComponent)
  (Audio|Components|Audio|FadeIn (Variables|Default|GetChaseMusicAudio) _fadeindurationchase 1.0 0.0 "Linear" :!class /Script/Engine.AudioComponent))

(fn SetChaseEffectAmount
  (params (EnemyDistance :type Float%20%28double-precision%29))
  (bind _chaseeffectstartdistance (Variables|Default|GetChaseEffectStartDistance))
  (Audio|Parameter|SetFloatParameter (Variables|Default|GetChaseMusicAudio) "EffectAmount" (- 1.0 (/ (Math|Float|Clamp(Float) EnemyDistance 5e+01 _chaseeffectstartdistance) _chaseeffectstartdistance)) :!class /Script/AudioExtensions.AudioParameterControllerInterface))

(fn Death
  (Audio|Components|Audio|FadeOut (Variables|Default|GetChaseMusicAudio) (Variables|Default|GetDeathFadeOutDuration) 0.0 "Linear" :!class /Script/Engine.AudioComponent))