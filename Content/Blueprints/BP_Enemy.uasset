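; Enemy pawn that roams the navmesh, chases the player and signals when the player is caught, while spawning BP_Rat AI at random intervals.
; Notice and kill colliders trigger chase and capture; chasing raises walk speed and repeats move requests, falling back to the player's navmesh-projected position.
; Hiding collider events stop or re-enable chasing; leaving the chase collider does nothing.
; A looping timeline bobs the mesh vertically.
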(event OnComponentBeginOverlap(NoticeCollider)
  (params (OverlappedComponent :type Primitive%20Component%20Object%20Reference) (OtherActor :type Actor%20Object%20Reference) (OtherComp :type Primitive%20Component%20Object%20Reference) (OtherBodyIndex :type Integer) (bFromSweep :type Boolean) (SweepResult :type Hit%20Result%20Structure%20%28by%20ref%29))
  ;[1 0.202 0] Collider actions
  (if (== (Utilities|GetClass OtherActor) "/Game/Blueprints/BP_FirstPersonCharacter.BP_FirstPersonCharacter_C")
    (CallFunction|StartChase)))

(event OnComponentBeginOverlap(KillCollider)
  (params (OverlappedComponent :type Primitive%20Component%20Object%20Reference) (OtherActor :type Actor%20Object%20Reference) (OtherComp :type Primitive%20Component%20Object%20Reference) (OtherBodyIndex :type Integer) (bFromSweep :type Boolean) (SweepResult :type Hit%20Result%20Structure%20%28by%20ref%29))
  ;[1 0.202 0] Collider actions
  (if (== (Utilities|GetClass OtherActor) "/Game/Blueprints/BP_FirstPersonCharacter.BP_FirstPersonCharacter_C")
    (CallFunction|PlayerCaught)))

(event OnComponentEndOverlap(ChaseCollider)
  (params (OverlappedComponent :type Primitive%20Component%20Object%20Reference) (OtherActor :type Actor%20Object%20Reference) (OtherComp :type Primitive%20Component%20Object%20Reference) (OtherBodyIndex :type Integer))
  ;[1 0.202 0] Collider actions
  (if (== (Utilities|GetClass OtherActor) "/Game/Blueprints/BP_FirstPersonCharacter.BP_FirstPersonCharacter_C")
    _))

(event Custom|Random%20Roam
  ;[0 0.7623 1] AI Movement
  (Utilities|FlowControl|ForLoopwithBreak 0 20 :!label _label
    (:LoopBody
      (bind _output_get (Variables|Default|SetRandomPoint (.RandomLocation (AI|Navigation|GetRandomReachablePointinRadius (Transformation|GetActorLocation) 5e+03 0 0))))
      (if (> (Math|Vector|Distance(Vector) _output_get (Transformation|GetActorLocation)) 2e+03)
        (goto _label Break)))
    (:Completed
      (AI|AIMoveTo self (Variables|Default|GetRandomPoint) 0 5.0 false
        (:OnSuccess
          (CallFunction|RandomRoam))))))

(event Custom|StartChase
  (bind _returnvalue (Game|GetPlayerCharacter 0))
  ;[0 0.7623 1] AI Movement
  (if (and (not (Variables|Default|GetIsChasing?)) (Variables|Default|GetCanChase?))
    (Variables|Default|SetIsChasing? true)
    (Variables|/Script/Engine.CharacterMovementComponent|SetMaxWalkSpeed (Variables|Character|GetCharacterMovement) (Variables|Default|GetChaseMaxWalkSpeed))
    (AI|AIMoveTo self "0, 0, 0" _returnvalue 5.0 false :!label _label
      (:OnSuccess
        _)
      (:OnFail
        (bind _returnvalue_2 (Actor|GetActorOfClass "/Script/NavigationSystem.RecastNavMesh"))
        (AI|AIMoveTo self (.ProjectedLocation (AI|Navigation|ProjectPointtoNavigation (Transformation|GetWorldLocation (Variables|/Script/Engine.Character|GetCapsuleComponent _returnvalue)) _returnvalue_2 0 "0, 0, 0")) 0 5.0 false
          (:OnSuccess
            _)
          (:OnFail
            _))))
    (Utilities|FlowControl|Delay 0.2)
    (if (Variables|Default|GetIsChasing?)
      (goto _label))))

(event Custom|StopChase
  ;[0 0.7623 1] AI Movement
  (if (Variables|Default|GetIsChasing?)
    (Variables|Default|SetIsChasing? false)
    (Variables|/Script/Engine.CharacterMovementComponent|SetMaxWalkSpeed (Variables|Character|GetCharacterMovement) (Variables|Default|GetOGMaxWalkSpeed))
    (CallFunction|RandomRoam)))

(event Custom|PlayerCaught
  ;[0 0.7623 1] AI Movement
  (if (not (Variables|Default|GetIsPlayerCaught?))
    (Variables|Default|SetIsPlayerCaught? true)
    (AI|AIMoveTo 0 "0, 0, 0" (Game|GetPlayerCharacter 0) 5.0 false
      (:then
        (Default|CallOnPlayerCaught)))))

(event Custom|DisableChase
  ;[1 1 0] BeginPlay
  (CallFunction|StopChase)
  (Variables|Default|SetCanChase? false))

(event Custom|EnableChase
  ;[1 1 0] BeginPlay
  (Variables|Default|SetCanChase? true))

(event Custom|StartWobble
  (bind _ogmeshtransform (Variables|Default|GetOGMeshTransform))
  (bind _returnvalue (Math|Transform|TransformLocation _ogmeshtransform "0, 0, 0"))
  (bind _halfsine (Timeline|Timeline PlayFromStart)
    (:Update
      (Transformation|SetRelativeLocation (Variables|Character|GetMesh) (Math|Vector|MakeVector (.x _returnvalue) (.y _returnvalue) (Math|Float|Lerp (.z _returnvalue) (+ (.z _returnvalue) 3e+01) _halfsine)) false false))
    (:Finished
      (if true
        (Timeline|Timeline PlayFromStart)))))

(event Custom|StartSpawningRats
  (bind _ratspawnlocation (Variables|Default|GetRatSpawnLocation))
  (AI|SpawnAIFromClass "/Game/Blueprints/BP_Rat.BP_Rat_C" 0 (Transformation|GetWorldLocation _ratspawnlocation) (Transformation|GetWorldRotation _ratspawnlocation) false 0 :!label _label)
  (Utilities|FlowControl|Delay (Math|Random|RandomFloatinRange (Variables|Default|GetRatSpawnRateMin) (Variables|Default|GetRatSpawnRateMax)))
  (goto _label))

(event EventBeginPlay
  ;[1 1 0] BeginPlay
  (CallFunction|RandomRoam)
  (bind _outactors (Actor|GetAllActorsOfClass "/Game/Blueprints/BP_HidingCollider.BP_HidingCollider_C"))
  (for _array_element _outactors
    (EventDispatchers|BindEventtoOnPlayerHide _array_element (delegate Custom|DisableChase))
    (EventDispatchers|BindEventtoOnPlayerStopHide _array_element (delegate Custom|EnableChase))
    (Variables|Default|SetOGMeshTransform (Transformation|GetRelativeTransform (Variables|Character|GetMesh)))
    (CallFunction|StartWobble)
    (Variables|Default|SetOGMaxWalkSpeed (Variables|/Script/Engine.CharacterMovementComponent|GetMaxWalkSpeed (Variables|Character|GetCharacterMovement)))
    (CallFunction|StartSpawningRats)))

(fn ConstructionScript)