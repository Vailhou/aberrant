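; AC_Activatable is an actor component that switches its owner on or off through BPI_Activatable, based on the states of other actors' AC_Activator components.
; On BeginPlay it binds to activators in RequiredToBeOn and, nested within that loop, RequiredToBeOff.
; Their events maintain a shared On collection.
; TryActivate activates the owner when all required and no unwanted activators are on, while a violating change deactivates it immediately.
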(event Custom|AddRequired
  (params (NewParam :type AC%20Activator%20Object%20Reference))
  (Utilities|Array|Add (Variables|Default|GetOn) NewParam)
  (CallFunction|TryActivate))

(event Custom|RemoveRequired
  (params (NewParam :type AC%20Activator%20Object%20Reference))
  (Utilities|Array|RemoveItem (Variables|Default|GetOn) NewParam)
  (Default|Deactivate (Variables|Default|GetActivatable)))

(event Custom|AddUnwanted
  (params (NewParam :type AC%20Activator%20Object%20Reference))
  (Utilities|Array|Add (Variables|Default|GetOn) NewParam)
  (Default|Deactivate (Variables|Default|GetActivatable)))

(event Custom|RemoveUnwanted
  (params (NewParam :type AC%20Activator%20Object%20Reference))
  (Utilities|Array|RemoveItem (Variables|Default|GetOn) NewParam)
  (CallFunction|TryActivate))

(event EventBeginPlay
  (bind _asbpi_activatable (Utilities|Casting|CastToBPI_Activatable (Components|GetOwner)))
  (Variables|Default|SetActivatable _asbpi_activatable)
  (for _array_element (Variables|Default|GetRequiredToBeOn)
    (EventDispatchers|BindEventtoOnSetActivateon (Actor|GetComponentbyClass _array_element "/Game/Blueprints/AC_Activator.AC_Activator_C") (delegate Custom|AddRequired))
    (EventDispatchers|BindEventtoOnSetActivateOff (Actor|GetComponentbyClass _array_element "/Game/Blueprints/AC_Activator.AC_Activator_C") (delegate Custom|RemoveRequired))
    (for _array_element_2 (Variables|Default|GetRequiredToBeOff)
      (EventDispatchers|BindEventtoOnSetActivateon (Actor|GetComponentbyClass _array_element_2 "/Game/Blueprints/AC_Activator.AC_Activator_C") (delegate Custom|AddUnwanted))
      (EventDispatchers|BindEventtoOnSetActivateOff (Actor|GetComponentbyClass _array_element_2 "/Game/Blueprints/AC_Activator.AC_Activator_C") (delegate Custom|RemoveUnwanted)))))

(fn TryActivate
  (for _array_element (Variables|Default|GetOn)
    (bind _array_element_2 (Utilities|Array|ForEachLoopwithBreak (Variables|Default|GetRequiredToBeOn))
      (:LoopBody
        (if (not (Utilities|Array|ContainsItem (Variables|Default|GetOn) (Actor|GetComponentbyClass _array_element_2 "/Game/Blueprints/AC_Activator.AC_Activator_C")))
          (return)))
      (:Completed
        (bind _array_element_3 (Utilities|Array|ForEachLoopwithBreak (Variables|Default|GetRequiredToBeOff))
          (:LoopBody
            (if (Utilities|Array|ContainsItem (Variables|Default|GetOn) (Actor|GetComponentbyClass _array_element_3 "/Game/Blueprints/AC_Activator.AC_Activator_C"))
              (return)))
          (:Completed
            (Default|Activate (Variables|Default|GetActivatable))
            (return)))))))