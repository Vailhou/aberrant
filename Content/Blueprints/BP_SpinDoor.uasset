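; BP_SpinDoor is an activatable door that swings open by rotating its Cylinder component around yaw.
; Activate plays the DoorOpen timeline, scaled by PlayTime, and Deactivate reverses it, with optional automatic closing when it finishes.
; Each update sets Cylinder yaw twice: first toward the Arrow's yaw, then from its starting yaw toward a hardcoded angle, which overrides the first.
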(event EventDeactivate
  (bind _amount (Timeline|DoorOpen Reverse)
    (:Update
      (Transformation|SetRelativeRotation (Variables|Default|GetCylinder) (Math|Rotator|MakeRotator 0.0 0.0 (Math|Float|Lerp 0.0 (.yaw (Variables|/Script/Engine.SceneComponent|GetRelativeRotation (Variables|Default|GetArrow))) _amount)) false false)
      (Transformation|SetRelativeRotation (Variables|Default|GetCylinder) (Math|Rotator|MakeRotator 0.0 0.0 (Math|Float|Lerp (.yaw (Variables|Default|GetChainOGRotation)) -182.0 _amount)) false false))
    (:Finished
      (if (Variables|Default|GetAutoCloseAfterOperning?)
        (CallFunction|Deactivate)))))

(event EventActivate
  (bind _amount (Timeline|DoorOpen Play)
    (:Update
      (Transformation|SetRelativeRotation (Variables|Default|GetCylinder) (Math|Rotator|MakeRotator 0.0 0.0 (Math|Float|Lerp 0.0 (.yaw (Variables|/Script/Engine.SceneComponent|GetRelativeRotation (Variables|Default|GetArrow))) _amount)) false false)
      (Transformation|SetRelativeRotation (Variables|Default|GetCylinder) (Math|Rotator|MakeRotator 0.0 0.0 (Math|Float|Lerp (.yaw (Variables|Default|GetChainOGRotation)) -182.0 _amount)) false false))
    (:Finished
      (if (Variables|Default|GetAutoCloseAfterOperning?)
        (CallFunction|Deactivate)))))

(event EventBeginPlay
  (Components|Timeline|SetPlayRate (Variables|Default|GetDoorOpen) (/ 1.0 (Variables|Default|GetPlayTime)))
  (Variables|Default|SetChainOGRotation (Variables|/Script/Engine.SceneComponent|GetRelativeRotation (Variables|Default|GetCylinder))))

(fn ConstructionScript)