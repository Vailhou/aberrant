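; Laser emitter actor that casts a bouncing beam to activate BP_GoalSphere targets.
; BeginPlay pools cylinder mesh actors; each Tick chains line traces from the arrow, stretching a cylinder along each segment and hiding unused ones.
; Bounces continue only off BPI_Reflective actors, along the hit normal rather than a mirrored angle, up to BounceAmount.
; A goal hit stops the chain; the goal deactivates when the beam leaves.
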(event EventBeginPlay
  (for _index (range 0 (Variables|Default|GetBounceAmount))
    (bind _returnvalue (Game|SpawnActorfromClass "/Script/Engine.StaticMeshActor" (Transformation|GetWorldTransform (Variables|Default|GetDefaultSceneRoot)) "Undefined" "MultiplyWithRoot" 0 0))
    (Components|StaticMesh|SetStaticMesh (Variables|/Script/Engine.StaticMeshActor|GetStaticMeshComponent _returnvalue) "/Game/Meshes/SM_LaserCylinder.SM_LaserCylinder")
    (Transformation|SetMobility _returnvalue "Movable")
    (Utilities|Array|Add (Variables|Default|GetLaserMeshes) _returnvalue)))

(event Collision|EventActorBeginOverlap
  (params (OtherActor :type Actor%20Object%20Reference)))

(event EventTick
  (params (DeltaSeconds :type Float%20%28single-precision%29))
  (bind _arrow (Variables|Default|GetArrow))
  (Variables|Default|SetIsActivating? false)
  (Variables|Default|SetPreviousHit "")
  (CallFunction|BounceLaser (Transformation|GetWorldLocation _arrow) (Math|Vector|GetForwardVector _arrow))
  (CallFunction|CheckifHittingGoal)
  (for _index (range 1 (Variables|Default|GetBounceAmount))
    (if (and (Variables|Default|GetPreviousReturn) (Utilities|DoesObjectImplementInterface (.HitActor (Collision|BreakHitResult (Variables|Default|GetPreviousHit))) "/Game/Blueprints/BPI_Reflective.BPI_Reflective_C"))
      (CallFunction|BounceLaser (.Location (Collision|BreakHitResult (Variables|Default|GetPreviousHit))) (.Normal (Collision|BreakHitResult (Variables|Default|GetPreviousHit))) _index)
      (CallFunction|CheckifHittingGoal)
      (else
        (CallFunction|HideLaserMesh _index))))
  (if (not (Variables|Default|GetIsActivating?))
    (Utilities|IsValid (Variables|Default|GetCurrentGoalSphere)
      (:Is%20Valid
        (Default|EndActivation (Variables|Default|GetCurrentGoalSphere))
        (Variables|Default|SetCurrentGoalSphere 0)))))

(fn ConstructionScript)

(fn AddLaserMesh
  (params (StartLocation :type Vector%20%28by%20ref%29) (EndLocation :type Vector%20%28by%20ref%29) (Index :type Integer))
  (bind _lasermeshes (Variables|Default|GetLaserMeshes))
  (bind _output (Utilities|Array|Get(acopy) _lasermeshes Index))
  (bind _staticmeshcomponent (Variables|/Script/Engine.StaticMeshActor|GetStaticMeshComponent _output))
  (bind _returnvalue (Transformation|GetWorldScale _staticmeshcomponent))
  (Transformation|SetWorldLocationAndRotation _staticmeshcomponent StartLocation (Math|Rotator|FindLookatRotation StartLocation EndLocation) false false)
  (Transformation|SetRelativeScale3D _staticmeshcomponent (Math|Vector|MakeVector (/ (Math|Vector|Distance(Vector) EndLocation StartLocation) 5e+01) (.y _returnvalue) (.z _returnvalue)))
  (Rendering|SetActorHiddenInGame _output false))

(fn BounceLaser
  (params (StartLocation :type Vector) (Direction :type Vector) (Index :type Integer))
  (bind _returnvalue (* Direction 1e+04))
  (bind _returnvalue_2 (+ StartLocation _returnvalue))
  (bind (_outhit _returnvalue_3) (Collision|LineTraceByChannel StartLocation _returnvalue_2 "TraceTypeQuery1" false (Utilities|Array|MakeArray (.HitActor (Collision|BreakHitResult (Variables|Default|GetPreviousHit)))) "None"))
  (Variables|Default|SetPreviousHit _outhit)
  (Variables|Default|SetPreviousReturn _returnvalue_3)
  (if _returnvalue_3
    (CallFunction|AddLaserMesh (.TraceStart (Collision|BreakHitResult _outhit)) (.Location (Collision|BreakHitResult _outhit)) Index)
    (else
      (CallFunction|AddLaserMesh StartLocation _returnvalue_2 Index))))

(fn HideLaserMesh
  (params (Index :type Integer))
  (Rendering|SetActorHiddenInGame (Utilities|Array|Get(acopy) (Variables|Default|GetLaserMeshes) Index) true))

(fn CheckifHittingGoal
  (bind _asbp_goal_sphere (Utilities|Casting|CastToBP_GoalSphere (.HitActor (Collision|BreakHitResult (Variables|Default|GetPreviousHit)))))
  (Default|StartActivation _asbp_goal_sphere)
  (Variables|Default|SetPreviousReturn false)
  (Variables|Default|SetCurrentGoalSphere _asbp_goal_sphere)
  (Variables|Default|SetIsActivating? true))