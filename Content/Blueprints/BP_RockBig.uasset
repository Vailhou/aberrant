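; BP_RockBig is a large rock that plays a dragging sound while it moves.
; Each tick it compares its velocity magnitude to MinAudibleDraggingSpeed, starting the Audio component if it is not already playing and stopping it below that threshold.
; The construction script is empty.
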(event EventTick
  (params (DeltaSeconds :type Float%20%28single-precision%29))
  (bind _audio (Variables|Default|GetAudio))
  (if (>= (Math|Vector|VectorLength (Transformation|GetVelocity)) (Variables|Default|GetMinAudibleDraggingSpeed))
    (if (not (Audio|Components|Audio|IsPlaying _audio))
      (Audio|Components|Audio|Play _audio 0.0))
    (else
      (Audio|Components|Audio|Stop _audio))))

(fn ConstructionScript)