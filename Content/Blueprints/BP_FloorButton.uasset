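; BP_FloorButton is a pressure button that stays active while the first-person character or a physics-simulating object rests on it.
; Collision box overlaps play or reverse a timeline that lowers the cube slightly, and tell ACActivator to start or stop activation.
; Before releasing, an overlap check confirms that no player or physics object remains on top.
; Disconnected loops using BPI_Activatable on ActivateObjects remain unused in the event graph.
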(event OnComponentBeginOverlap(CollisonBox)
  (params (OverlappedComponent :type Primitive%20Component%20Object%20Reference) (OtherActor :type Actor%20Object%20Reference) (OtherComp :type Primitive%20Component%20Object%20Reference) (OtherBodyIndex :type Integer) (bFromSweep :type Boolean) (SweepResult :type Hit%20Result%20Structure%20%28by%20ref%29))
  (if (or (== (Utilities|GetClass OtherActor) "/Game/Blueprints/BP_FirstPersonCharacter.BP_FirstPersonCharacter_C") (Physics|IsSimulatingPhysics OtherComp "None"))
    (Variables|Default|SetIsActive? true)
    (CallFunction|DownAnimation)
    (Default|StartActivation (Variables|Default|GetAC_Activator))))

(event OnComponentEndOverlap(CollisonBox)
  (params (OverlappedComponent :type Primitive%20Component%20Object%20Reference) (OtherActor :type Actor%20Object%20Reference) (OtherComp :type Primitive%20Component%20Object%20Reference) (OtherBodyIndex :type Integer))
  (if (and (or (== (Utilities|GetClass OtherActor) "/Game/Blueprints/BP_FirstPersonCharacter.BP_FirstPersonCharacter_C") (Physics|IsSimulatingPhysics OtherComp "None")) (CallFunction|AreThereNotAnyObjectsonTopOfButton))
    (Variables|Default|SetIsActive? false)
    (CallFunction|UpAnimation)
    (Default|StopActivation (Variables|Default|GetAC_Activator))))

(event Custom|DownAnimation
  (bind _zoffset (Timeline|ButtonDown Play)
    (:Update
      (Transformation|SetRelativeLocation (Variables|Default|GetCube) (Math|Vector|MakeVector 0.0 0.0 (Math|Float|Lerp (Variables|Default|GetButtonOGLocationZ) (- (Variables|Default|GetButtonOGLocationZ) 5.0) _zoffset)) false false))))

(event Custom|UpAnimation
  (bind _zoffset (Timeline|ButtonDown Reverse)
    (:Update
      (Transformation|SetRelativeLocation (Variables|Default|GetCube) (Math|Vector|MakeVector 0.0 0.0 (Math|Float|Lerp (Variables|Default|GetButtonOGLocationZ) (- (Variables|Default|GetButtonOGLocationZ) 5.0) _zoffset)) false false))))

(event EventBeginPlay
  (Variables|Default|SetButtonOGLocationZ (.z (Variables|/Script/Engine.SceneComponent|GetRelativeLocation (Variables|Default|GetCube)))))

(fn ConstructionScript)

(fn AreThereNotAnyObjectsonTopOfButton
  ;[1 1 1] No physicsobject on top of button
  (for _array_element (Class|PrimitiveComponent|GetOverlappingComponents (Variables|Default|GetCollisonBox))
    (if (Physics|IsSimulatingPhysics _array_element "None")
      (LocalVariables|SetIsPhysicsObjectOnTopOfButton? true)))
  (return (and (not (LocalVariables|GetIsPhysicsObjectOnTopOfButton?)) (== (Utilities|Array|Length (Collision|GetOverlappingActors (Variables|Default|GetCollisonBox) "/Game/Blueprints/BP_FirstPersonCharacter.BP_FirstPersonCharacter_C" :!class /Script/Engine.PrimitiveComponent)) 0))))